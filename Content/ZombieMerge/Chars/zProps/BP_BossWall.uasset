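; BP_BossWall is a destructible boss wall prop that loses health when damaged and swaps to a destroyed version.
; AnyDamage lowers WallHealth and spawns sand impact VFX, or clears StillAlive when the hit would deplete health.
; Tick polls that flag and, once, stores BossWall-tagged actors in BikerRef and calls DestroyWallEvent.
; That event retags the wall as Killed, spawns the SelectSpawnDestr class in its place and destroys the actor.
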(event Custom|DestroyWallEvent
  (bind _bosswall (Variables|Default|GetBossWall))
  (Utilities|FlowControl|Sequence
    (:then_0
      (Variables|Default|SetWorldLoc (Transformation|GetWorldLocation _bosswall))
      (Components|DestroyComponent _bosswall)
      (Variables|Default|SetTags (Utilities|Array|MakeArray "Killed" "Killed"))
      (Game|SpawnActorfromClass (Variables|Default|GetSelect%20Spawn%20Destr) (Math|Transform|MakeTransform (Variables|Default|GetWorldLoc) "0, 0, 0" "1.000000,1.000000,1.000000") "Undefined" 0 0)
      (Actor|DestroyActor))
    (:then_1
      (Development|PrintString "DestroyingBOSS_WALL"))))

(event Game|Damage|EventAnyDamage
  (params (Damage :type Float%20%28single-precision%29) (DamageType :type Damage%20Type%20Object%20Reference) (InstigatedBy :type Controller%20Object%20Reference) (DamageCauser :type Actor%20Object%20Reference))
  (bind _bosswall (Variables|Default|GetBossWall))
  (bind _returnvalue (Transformation|GetWorldLocation _bosswall))
  (Utilities|FlowControl|Sequence
    (:then_0
      (if (Variables|Default|GetStillAlive?)
        (Variables|Default|SetWorldLoc (Transformation|GetWorldLocation (Variables|Default|GetBossWall)))
        (if (<= (- (Variables|Default|GetWallHealth) Damage) 0.0)
          (Variables|Default|SetStillAlive? false)
          (else
            (Variables|Default|SetWallHealth (Math|Float|Truncate (- (Variables|Default|GetWallHealth) Damage)))
            (Effects|SpawnEmitteratLocation "/Game/bulletvfx/Particles/VFX_Impact_SandMassive.VFX_Impact_SandMassive" (Math|Vector|MakeVector (.x _returnvalue) (.y _returnvalue) (+ (.z _returnvalue) 5e+01)) "90.000000, 0, 0" "1.000000,1.000000,1.000000" true "AutoRelease")
            (Utilities|FlowControl|Sequence)))
        (else
          (Variables|Default|SetStillAlive? false))))
    (:then_1
      (Development|PrintString (Utilities|String|ToString(Float) Damage) true true "(R=0.472253,G=0.000000,B=0.510417,A=1.000000)"))))

(event EventTick
  (params (DeltaSeconds :type Float%20%28single-precision%29))
  (if (not (Variables|Default|GetStillAlive?))
    (Utilities|FlowControl|DoOnce false
      (:Completed
        (bind _outactors (Actor|GetAllActorswithTag "BossWall"))
        (Variables|Default|SetBikerRef _outactors)
        (CallFunction|DestroyWallEvent)))))

(fn ConstructionScript)