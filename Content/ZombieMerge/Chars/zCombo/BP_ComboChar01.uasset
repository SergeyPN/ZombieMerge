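; Combo character in ZombieMerge that autonomously fights enemies, spawning a ground crack effect on BeginPlay.
; Once Ready2Fight is set, an event-driven loop picks the nearest Enemy1 actor, approaches via AIMoveTo at randomized speed, and attacks on a timed delay.
; It retargets when a wall or enemy's StillAlive clears, switching to the BossWall when no enemies remain.
; With no targets left, it randomly stops or wanders nearby, flagging AllEnemiesDead.
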(event Custom|DestroyBossWallEvent
  ;[1 1 1] DestroyBossWallEvent
  (Utilities|FlowControl|Sequence
    (:then_0
      (Utilities|FlowControl|DoOnce false
        (:Completed
          (Variables|Default|SetAttackBW true)
          (bind _outactors (Actor|GetAllActorswithTag "BossWall"))
          (Variables|Default|SetCloserEnemy (Utilities|Array|Get(acopy) _outactors))
          (Utilities|IsValid (Variables|Default|GetCloserEnemy)
            (:Is%20Valid
              (Variables|Default|SetCurrEnemyLoc (Transformation|GetActorLocation (Variables|Default|GetCloserEnemy))))))))
    (:then_1
      (Utilities|IsValid (Variables|Default|GetCloserEnemy)
        (:Is%20Valid
          (CallFunction|MovetoEnemyEvent))))))

(event Custom|PlaceCrackFXEvent
  (bind _capsulecomponent (Variables|Collision|GetCapsuleComponent))
  (bind _returnvalue (Transformation|GetWorldLocation _capsulecomponent))
  ;[1 1 1] PlaceCrackFXEvent
  (bind _outhit (Collision|LineTraceByChannel _returnvalue (- _returnvalue "0,0,10000.000000") "TraceTypeQuery1" false 0 "None"))
  (Game|SpawnActorfromClass "/Game/ZombieMerge/Chars/BP_CrackFX.BP_CrackFX_C" (Math|Transform|MakeTransform (.Location (Collision|BreakHitResult _outhit)) "0, 0, 0" "1.000000,1.000000,1.000000") "Undefined" 0 0))

(event Custom|MoveToEnemyEvent
  ;[1 1 1] MoveToEnemyEvent
  (Variables|Default|SetIsMoving? true)
  (Variables|/Script/Engine.CharacterMovementComponent|SetMaxWalkSpeed (Variables|Character|GetCharacterMovement) (Math|Random|RandomFloatinRange 2.2e+02 3e+02))
  (AI|AIMoveTo self (.RandomLocation (AI|Navigation|GetRandomReachablePointinRadius (Variables|Default|GetCurrEnemyLoc) 25.0 0 0)) 0 1.5e+02 false ; MoveTo
    (:OnSuccess
      (CallFunction|AttackingEvent))
    (:OnFail
      (CallFunction|FindEnemiesEvent))))

(event Custom|AllEnemiesDeadEvent
  ;[1 1 1] AllEnemiesDeadEvent
  (if (Math|Random|RandomBool)
    (Variables|/Script/Engine.CharacterMovementComponent|SetMaxWalkSpeed (Variables|Character|GetCharacterMovement) 0.0)
    (Variables|Default|SetAllEnemiesDead true)
    (else
      (CallFunction|WalkRandomPlaceEvent))))

(event Custom|WalkRandomPlaceEvent
  ;[1 1 1] WalkRandomPlace
  (Variables|/Script/Engine.CharacterMovementComponent|SetMaxWalkSpeed (Variables|Character|GetCharacterMovement) (Math|Random|RandomFloatinRange 2e+02 3e+02))
  (Utilities|FlowControl|Delay (Math|Random|RandomFloatinRange 0.2 0.5))
  (AI|AIMoveTo self (.RandomLocation (AI|Navigation|GetRandomReachablePointinRadius (Transformation|GetActorLocation) 2.5e+02 0 0)) 0 5.0 false
    (:OnSuccess
      (Variables|Default|SetAllEnemiesDead true))
    (:OnFail
      (CallFunction|WalkRandomPlaceEvent))))

(event Custom|FindEnemiesEvent
  ;[1 1 1] FindEnemiesEvent
  (Variables|Default|SetNearDistance 1e+06)
  (Utilities|FlowControl|Delay 0.2)
  (bind _outactors (Actor|GetAllActorswithTag "Enemy1"))
  (if (Utilities|Array|IsNotEmpty _outactors)
    (bind _output_get (Variables|Default|SetMyEnemiesArray _outactors))
    (for _array_element _output_get
      (if (< (Math|Vector|Distance(Vector) (Transformation|GetActorLocation _array_element) (Transformation|GetWorldLocation (Variables|Character|GetMesh))) (Variables|Default|GetNearDistance))
        (bind _output_get_2 (Variables|Default|SetCloserEnemy _array_element))
        (Variables|Default|SetCurrEnemyLoc (Transformation|GetActorLocation _output_get_2))
        (Variables|Default|SetNearDistance (Math|Vector|Distance(Vector) (Transformation|GetActorLocation _array_element) (Transformation|GetWorldLocation (Variables|Character|GetMesh))))))
    (Utilities|FlowControl|Sequence
      (:then_0
        (Utilities|IsValid (Variables|Default|GetCloserEnemy)
          (:Is%20Valid
            (CallFunction|MovetoEnemyEvent))
          (:Is%20Not%20Valid
            (CallFunction|FindEnemiesEvent))))
      (:then_1))
    (else
      (Utilities|FlowControl|Sequence
        (:then_0
          (CallFunction|DestroyBossWallEvent))
        (:then_1
          (Utilities|IsValid (Variables|Default|GetCloserEnemy)
            (:Is%20Not%20Valid
              (Utilities|FlowControl|DoOnce false
                (:Completed
                  (CallFunction|AllEnemiesDeadEvent))))))))))

(event Custom|AttackingEvent
  (bind _closerenemy (Variables|Default|GetCloserEnemy))
  (bind _closerenemy_2 (Variables|Default|GetCloserEnemy))
  ;[1 1 1] Attacking
  (if (or (Actor|ActorHasTag _closerenemy_2 "Enemy1") (Actor|ActorHasTag _closerenemy_2 "BossWall"))
    (Variables|Default|SetAttacking true)
    (Variables|/Script/Engine.CharacterMovementComponent|SetMaxWalkSpeed (Variables|Character|GetCharacterMovement) 0.0)
    (Transformation|SetActorRotation (Math|Rotator|MakeRotator 0.0 0.0 (.yaw (Math|Rotator|FindLookatRotation (Transformation|GetActorLocation) (Transformation|GetActorLocation (Variables|Default|GetCloserEnemy))))))
    (Utilities|FlowControl|Delay (Variables|Default|GetAttackingAnimTime))
    (Variables|Default|SetAttacking false)
    (Variables|/Script/Engine.CharacterMovementComponent|SetMaxWalkSpeed (Variables|Character|GetCharacterMovement) (Math|Random|RandomFloatinRange 1.5e+02 3e+02))
    (Utilities|IsValid _closerenemy
      (:Is%20Valid
        (if (Variables|Default|GetAttackBW)
          (Utilities|FlowControl|Sequence
            (:then_0
              (CallFunction|AttackingEvent))
            (:then_1))
          (else
            (Utilities|FlowControl|Sequence :!pinned true ; Need New Enemy here
              (:then_0
                (bind _asbp_walls (Utilities|Casting|CastToBP_Walls _closerenemy))
                (if (Variables|/Game/ZombieMerge/Chars/zProps/BP_Walls.BP_Walls_C|GetStillAlive? _asbp_walls)
                  (Utilities|IsValid (Variables|Default|GetCloserEnemy)
                    (:Is%20Valid
                      (CallFunction|AttackingEvent))
                    (:Is%20Not%20Valid
                      (CallFunction|FindEnemiesEvent)))
                  (else
                    (CallFunction|FindEnemiesEvent))))
              (:then_1
                (bind _asbp_tame_enemy (Utilities|Casting|CastToBP_TameEnemy _closerenemy))
                (if (Variables|/Game/ZombieMerge/Chars/zTame/BP_TameEnemy.BP_TameEnemy_C|GetStillAlive? _asbp_tame_enemy)
                  (Utilities|IsValid (Variables|Default|GetCloserEnemy)
                    (:Is%20Valid
                      (CallFunction|AttackingEvent))
                    (:Is%20Not%20Valid
                      (CallFunction|FindEnemiesEvent)))
                  (else
                    (CallFunction|FindEnemiesEvent))))
              (:then_2
                (bind _asbp_energy_enemy (Utilities|Casting|CastToBP_EnergyEnemy _closerenemy))
                (if (Variables|/Game/ZombieMerge/Chars/zEnegry/BP_EnergyEnemy.BP_EnergyEnemy_C|GetStillAlive? _asbp_energy_enemy)
                  (Utilities|IsValid (Variables|Default|GetCloserEnemy)
                    (:Is%20Valid
                      (CallFunction|AttackingEvent))
                    (:Is%20Not%20Valid
                      (CallFunction|FindEnemiesEvent)))
                  (else
                    (CallFunction|FindEnemiesEvent))))))))
      (:Is%20Not%20Valid
        (CallFunction|FindEnemiesEvent)))
    (elif (Variables|Default|GetAttackBW)
      (CallFunction|AllEnemiesDeadEvent)
      (else
        (CallFunction|FindEnemiesEvent)))))

(event EventBeginPlay
  (CallFunction|PlaceCrackFXEvent) ; Place Crack
)

(event EventTick
  (params (DeltaSeconds :type Float%20%28single-precision%29))
  (if (Variables|Default|GetReady2Fight)
    (Utilities|FlowControl|Sequence
      (:then_0
        (Utilities|FlowControl|DoOnce false
          (:Completed
            (CallFunction|FindEnemiesEvent) ; FindEnemies
          ))))))

(fn ConstructionScript)