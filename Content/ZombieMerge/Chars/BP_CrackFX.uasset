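; BP_CrackFX is a crack decal effect that appears with a dust burst when spawned.
; On BeginPlay it creates a dynamic instance of the crack decal material and animates its Dissolve parameter through an appearance timeline.
; It also randomizes the decal's scale and roll so repeated cracks vary, then spawns a dust explosion emitter at the decal's location.
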(event EventBeginPlay
  (bind _decal (Variables|Default|GetDecal))
  (Utilities|FlowControl|Sequence
    (:then_0
      (bind _returnvalue (Rendering|Material|CreateDynamicMaterialInstance "/Game/ZombieMerge/Mats/MI_Decal_Crack.MI_Decal_Crack" "None" "None" :!class /Script/Engine.KismetMaterialLibrary))
      (bind _output_get (Variables|Default|SetDynMatCrack _returnvalue))
      (Rendering|Components|Decal|SetDecalMaterial (Variables|Default|GetDecal) _output_get)
      (bind _maskanim (Timeline|TL_Appear Play)
        (:Update
          (Rendering|Material|SetScalarParameterValue (Variables|Default|GetDynMatCrack) "Dissolve" _maskanim :!class /Script/Engine.MaterialInstanceDynamic))))
    (:then_1
      (Transformation|SetWorldScale3D _decal (Math|Conversions|ToVector(Float) (Math|Random|RandomFloatinRange 0.8 1.2)))
      (Transformation|AddLocalRotation _decal (Math|Rotator|MakeRotator (Math|Random|RandomFloatinRange -1.8e+02 1.8e+02) 0.0 0.0) false false))
    (:then_2
      (Effects|SpawnEmitteratLocation "/Game/StarterContent/Particles/P_DustExp.P_DustExp" (Transformation|GetWorldLocation (Variables|Default|GetDecal))))))

(fn ConstructionScript)