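; Sheriff actor for ZombieMerge that periodically does a timed "yahoo" cheer until the boss wall is gone.
; A DoN loop with random delays fires the cheer up to CountYahoo times, each briefly raising LetsYahooSheriff and printing a debug string.
; BeginPlay caches the first BossWall-tagged actor, which a delayed Tick check polls for validity.
; Once that reference is invalid, WeWin is set, blocking further cheers.
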(event Custom|SheriffYahooEvent
  (if (not (Variables|Default|GetWeWin))
    (Variables|Default|SetLetsYahooSheriff true)
    (Utilities|FlowControl|Delay 3.0)
    (Variables|Default|SetLetsYahooSheriff false)
    (Development|PrintString "Sheriff Yahoo")))

(event EventBeginPlay
  ;[0.2654 1 0.7774] Do N Times with Delay
  (Utilities|FlowControl|Sequence
    (:then_0
      (bind _counter (Utilities|FlowControl|DoN (Variables|Default|GetCount%20Yahoo) :!label _label)
        (:Exit
          (CallFunction|SheriffYahooEvent)
          (Utilities|FlowControl|Delay (Math|Random|RandomFloatinRange 8.0 11.0))
          (if (== _counter (Variables|Default|GetCount%20Yahoo))
            (Utilities|FlowControl|Sequence
              (:then_1
                (goto _label Reset)))
            (else
              (goto _label))))))
    (:then_1
      (bind _outactors (Actor|GetAllActorswithTag "BossWall"))
      (Variables|Default|SetBossWallRef (Utilities|Array|Get(acopy) _outactors)))))

(event EventTick
  (params (DeltaSeconds :type Float%20%28single-precision%29))
  (Utilities|FlowControl|Delay 5.0)
  (Utilities|IsValid (Variables|Default|GetBossWallRef)
    (:Is%20Not%20Valid
      (Utilities|FlowControl|DoOnce false
        (:Completed
          (Variables|Default|SetLetsYahooSheriff false)
          (Variables|Default|SetWeWin true))))))

(fn ConstructionScript)