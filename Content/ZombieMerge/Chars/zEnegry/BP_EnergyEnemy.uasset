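; BP_EnergyEnemy is an enemy character that takes damage and marks itself dead when its health runs out.
; AnyDamage either reduces integer Health, spawns a flesh impact effect and sets IsGettingHit, or clears StillAlive on a lethal hit.
; Tick polls StillAlive, retags the dead actor as Killed and, through a DoOnce, clears the hit flag and fires KillEvent, which only replays the impact effect.
; The construction script initializes Tags from ActorTags.
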(event Custom|KillEvent
  (bind _worldloc (Variables|Default|GetWorldLoc))
  (Effects|SpawnEmitteratLocation "/Game/bulletvfx/Particles/VFX_Impact_Flesh.VFX_Impact_Flesh" (Math|Vector|MakeVector (.x _worldloc) (.y _worldloc) (+ (.z _worldloc) 5e+01)) "90.000000, 0, 0"))

(event EventTick
  (params (DeltaSeconds :type Float%20%28single-precision%29))
  (if (not (Variables|Default|GetStillAlive?))
    (Variables|Default|SetTags (Utilities|Array|MakeArray "Killed" "Killed"))
    (Utilities|FlowControl|DoOnce false
      (:Completed
        (Variables|Default|SetisGettingHit? false)
        (CallFunction|KillEvent)))))

(event Game|Damage|EventAnyDamage
  (params (Damage :type Float%20%28single-precision%29) (DamageType :type Damage%20Type%20Object%20Reference) (InstigatedBy :type Controller%20Object%20Reference) (DamageCauser :type Actor%20Object%20Reference))
  (Utilities|FlowControl|Sequence
    (:then_0
      (if (Variables|Default|GetStillAlive?)
        (Variables|Default|SetWorldLoc (Transformation|GetWorldLocation (Variables|Collision|GetCapsuleComponent)))
        (if (<= (- (Variables|Default|GetHealth) Damage) 0.0)
          (Variables|Default|SetStillAlive? false)
          (else
            (Variables|Default|SetHealth (Math|Float|Truncate (- (Variables|Default|GetHealth) Damage)))
            (Effects|SpawnEmitteratLocation "/Game/bulletvfx/Particles/VFX_Impact_Flesh.VFX_Impact_Flesh" (Math|Vector|MakeVector (.x (Variables|Default|GetWorldLoc)) (.y (Variables|Default|GetWorldLoc)) (+ (.z (Variables|Default|GetWorldLoc)) 5e+01)) "90.000000, 0, 0")
            (Variables|Default|SetisGettingHit? true)))
        (else
          (Variables|Default|SetStillAlive? false))))))

(fn ConstructionScript
  (Variables|Default|SetTags (Variables|Default|GetActorTags)))